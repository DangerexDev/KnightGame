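; Dialogue queue component that holds lines of dialogue and steps through them in order.
; QueueDialogue appends every row of a given data table to the queue as data table row handles.
; MoveToNextLine records the current line in History, advances the index and announces the new line.
; At the end of the queue it clears queue and history and signals completion, without resetting the index.
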(fn QueueDialogue
  (params (InDialogueLinesDataTable :type Data%20Table%20Object%20Reference))
  (bind _outrownames (DataTable|GetDataTableRowNames InDialogueLinesDataTable))
  (for _array_element _outrownames
    (Utilities|Array|Add (Variables|Queue|GetDialogueLinesQueue) (Utilities|Struct|MakeDataTableRowHandle InDialogueLinesDataTable _array_element))))

(fn MovetoNextLine
  (CallFunction|AddCurrentLinetoHistory)
  (bind _result (Math|Integer|IncrementInt (Variables|Queue|GetCurrentLineIndex))
    (:%20%20
      (if (== _result (Utilities|Array|Length (Variables|Queue|GetDialogueLinesQueue)))
        (Utilities|Array|Clear (Variables|Queue|GetDialogueLinesQueue))
        (Utilities|Array|Clear (Variables|History|GetHistory))
        (Default|CallOnFinished)
        (else
          (bind _output_get (Variables|Current|SetCurrentLine (Utilities|Array|Get(acopy) (Variables|Queue|GetDialogueLinesQueue) (Variables|Queue|GetCurrentLineIndex))))
          (Default|CallOnNewLine _output_get))))))

(fn AddCurrentLinetoHistory
  (Utilities|Array|Add (Variables|History|GetHistory) (Utilities|Array|Get(acopy) (Variables|Queue|GetDialogueLinesQueue) (Variables|Queue|GetCurrentLineIndex))))