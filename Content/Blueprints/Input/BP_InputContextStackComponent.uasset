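; Player controller component that manages Enhanced Input mapping contexts as a stack.
; Pushing adds a context and can remove the previous top from the local player subsystem.
; Popping removes the top context unless the one beneath is identical, then reactivates that one if inactive.
; BeginPlay pushes the default context, then appends the controlled KnightGameCharacter's default mapping context to the stack without activating it.
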(fn PushInputContext
  (params (bDisablePrevious :type Boolean) (MappingContext :type Input%20Mapping%20Context%20Object%20Reference))
  (Utilities|FlowControl|Sequence
    (:then_0
      (if bDisablePrevious
        (Input|RemoveMappingContext (PlayerController|LocalPlayerSubsystems|GetEnhancedInputLocalPlayerSubsystem (Variables|Player|GetPlayerController)) (Input|GetTopOfStack) "(bIgnoreAllPressedKeysUntilRelease=True,bForceImmediately=False)")))
    (:then_1
      (Utilities|Array|Add (Variables|Input|GetContextStack) MappingContext)
      (if (not (Input|IsContextActive MappingContext))
        (Input|AddMappingContext (PlayerController|LocalPlayerSubsystems|GetEnhancedInputLocalPlayerSubsystem (Variables|Player|GetPlayerController)) MappingContext 0 "(bIgnoreAllPressedKeysUntilRelease=True,bForceImmediately=False)")))))

(fn PopInputContext
  (bind _contextstack (Variables|Input|GetContextStack))
  (Utilities|FlowControl|Sequence
    (:then_0
      (LocalVariables|SetContextToPop (Input|GetTopOfStack)))
    (:then_1
      (Utilities|Array|RemoveIndex _contextstack (Utilities|Array|LastIndex _contextstack)))
    (:then_2
      (bind _output_get (LocalVariables|SetNewTopOfStack (Input|GetTopOfStack)))
      (if (!= _output_get (LocalVariables|GetContextToPop))
        (Input|RemoveMappingContext (PlayerController|LocalPlayerSubsystems|GetEnhancedInputLocalPlayerSubsystem (Variables|Player|GetPlayerController)) (LocalVariables|GetContextToPop) "(bIgnoreAllPressedKeysUntilRelease=True,bForceImmediately=False)")))
    (:then_3
      (if (not (Input|IsContextActive (LocalVariables|GetNewTopOfStack)))
        (Input|AddMappingContext (PlayerController|LocalPlayerSubsystems|GetEnhancedInputLocalPlayerSubsystem (Variables|Player|GetPlayerController)) (LocalVariables|GetNewTopOfStack) 0 "(bIgnoreAllPressedKeysUntilRelease=True,bForceImmediately=False)")))))

(fn GetTopOfStack
  (bind _contextstack (Variables|Input|GetContextStack))
  (return (Utilities|Array|Get(acopy) _contextstack (Utilities|Array|LastIndex _contextstack))))

(fn ReceiveBeginPlay
  (|CallParentFunction)
  (bind _output_get (Variables|Player|SetPlayerController (.AsPlayer%20Controller (Utilities|Casting|CastToPlayerController (Components|GetOwner)))))
  (Utilities|FlowControl|Sequence
    (:then_0
      (Input|PushInputContext true (Variables|Input|GetDefaultContext)))
    (:then_1
      (bind _asknight_game_character (Utilities|Casting|CastToKnightGameCharacter (Pawn|GetControlledPawn _output_get)))
      (Utilities|Array|Add (Variables|Input|GetContextStack) (Variables|/Script/KnightGame.KnightGameCharacter|GetDefaultMappingContext _asknight_game_character)))))

(fn IsContextActive
  (params (MappingContext :type Input%20Mapping%20Context%20Object%20Reference))
  (return (.ReturnValue (Class|EnhancedInputSubsystemInterface|HasMappingContext (PlayerController|LocalPlayerSubsystems|GetEnhancedInputLocalPlayerSubsystem (Variables|Player|GetPlayerController)) MappingContext))))