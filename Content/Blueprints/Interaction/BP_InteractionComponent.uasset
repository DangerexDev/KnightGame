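; Interaction component that makes its owning actor interactable by one interactor at a time.
; On BeginPlay it adds a sphere to the owner, sized by InteractRadius, that overlaps only a custom interaction collision channel.
; Interact instantiates the behavior class from InteractionData and delegates to it, ignoring calls while an interactor is active.
; When that behavior finishes, the component clears its state and fires its own OnFinished.
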(fn Interact
  (params (Interactor :type BP%20Interactor%20Component%20Object%20Reference))
  (Variables|Interaction|GetCurrentInteractor
    (:then)
    (:else
      (Variables|Interaction|SetCurrentInteractor Interactor)
      (bind _returnvalue (Game|ConstructObjectfromClass (Variables|/Game/Blueprints/Interaction/Data/BP_InteractionDataAsset.BP_InteractionDataAsset_C|GetInteractionBehavior (Variables|Interaction|GetInteractionData))))
      (bind _output_get (Variables|Interaction|SetActiveInteractionScript _returnvalue))
      (EventDispatchers|BindEventtoOnFinished _output_get (EventDispatchers|CreateEvent :!event ActiveInteractionScriptonFinished))
      (Default|Interact (Variables|Interaction|GetActiveInteractionScript) (Variables|Interaction|GetCurrentInteractor)))))

(fn FinishInteract
  (Variables|Interaction|SetCurrentInteractor 0)
  (Variables|Interaction|SetActiveInteractionScript 0)
  (Default|CallOnFinished))

(fn ActiveInteractionScriptonFinished
  (Interact|FinishInteract))

(fn ReceiveBeginPlay
  (|CallParentFunction)
  ;[1 1 1] TODO: Use a designer-specified collision volume instead.
  (bind _returnvalue (Game|AddComponentbyClass (Components|GetOwner) "/Script/Engine.SphereComponent" false))
  (Variables|Interaction|SetSphereCollisionComponent _returnvalue)
  (Components|Sphere|SetSphereRadius (Variables|Interaction|GetSphereCollisionComponent) (Variables|Interaction|GetInteractRadius) true)
  (Collision|SetCollisionResponsetoAllChannels (Variables|Interaction|GetSphereCollisionComponent) "ECR_Ignore")
  (Collision|SetCollisionResponsetoChannel (Variables|Interaction|GetSphereCollisionComponent) "ECC_GameTraceChannel1" "ECR_Overlap")
  (Collision|SetCollisionObjectType (Variables|Interaction|GetSphereCollisionComponent) "ECC_GameTraceChannel1"))