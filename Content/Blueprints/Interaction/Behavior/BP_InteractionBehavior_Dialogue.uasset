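; Interaction behavior that starts a dialogue sequence when a player interacts with its owner.
; Interact finds the dialogue queue component on the interacting player's HUD, binds to its finished event and queues a hardcoded sample Kaye dialogue table, marked to become dynamic.
; The behavior reports finished when the dialogue ends, or immediately if the interactor is not a player-controlled pawn.
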(fn Interact
  (params (InteractorComponent :type BP%20Interactor%20Component%20Object%20Reference))
  (|CallParentFunction InteractorComponent)
  (bind _aspawn (Utilities|Casting|CastToPawn (Components|GetOwner InteractorComponent))
    (:then
      (bind _asplayer_controller (Utilities|Casting|CastToPlayerController (Pawn|GetController _aspawn))
        (:then
          (bind _output_get (LocalVariables|SetDialogueQueueComponent (Actor|GetComponentbyClass (HUD|GetHUD _asplayer_controller) "/Game/Blueprints/Dialogue/BP_DialogueQueueComponent.BP_DialogueQueueComponent_C")))
          (EventDispatchers|BindEventtoOnFinished _output_get (EventDispatchers|CreateEvent :!event DialogueQueueComponentonFinished))
          ;[1 1 1] TODO: Make the table dynamic
          (Default|QueueDialogue (LocalVariables|GetDialogueQueueComponent) "/Game/Data/Dialogue/DialogueLines_Kaye_Sample.DialogueLines_Kaye_Sample"))
        (:CastFailed
          (Default|CallOnFinished :!label _label))))
    (:CastFailed
      (goto _label))))

(fn DialogueQueueComponentonFinished
  (Default|CallOnFinished))