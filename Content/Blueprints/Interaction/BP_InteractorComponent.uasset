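; Interactor component that lets its owner interact with nearby actors that have a BP_InteractionComponent.
; A child collision primitive tracks overlapping actors, and the one nearest the owner supplies the interaction candidate.
; The Interact input starts the candidate's interaction or ends the active one, as the candidate is cleared during an interaction.
; Overlap changes and interaction ends re-evaluate the candidate, with dispatchers announcing candidate and active interaction changes.
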(event Input|EnhancedActionEvents|EnhancedInputActionIA_Avatar_Interact
  (params (ActionValue :type Boolean) (ElapsedSeconds :type Float%20%28double-precision%29) (TriggeredSeconds :type Float%20%28double-precision%29) (InputAction :type Input%20Action%20Object%20Reference :default "/Game/Data/Input/Actions/IA_Avatar_Interact.IA_Avatar_Interact"))
  (:Completed
    (Interact|Interact)))

(fn ReceiveBeginPlay
  (|CallParentFunction)
  (Collision|DetermineCollision)
  (Collision|SetUpCollisionBindings))

(fn DetermineInteractionCandidate
  (Utilities|FlowControl|Sequence
    (:then_0
      (Variables|Candidate|GetActiveInteraction
        (:then
          (LocalVariables|SetNewInteractionCandidate 0))
        (:else
          (bind _output_get (LocalVariables|SetNearestActor (.ReturnValue (Actor|FindNearestActor (Transformation|GetActorLocation (Components|GetOwner)) (Variables|Collision|GetInRangeInteractionActors)))))
          (Utilities|IsValid _output_get
            (:Is%20Valid
              (LocalVariables|SetNewInteractionCandidate (Actor|GetComponentbyClass _output_get "/Game/Blueprints/Interaction/BP_InteractionComponent.BP_InteractionComponent_C")))))))
    (:then_1
      (if (!= (Variables|Candidate|GetInteractionCandidate) (LocalVariables|GetNewInteractionCandidate))
        (bind _output_get_2 (Variables|Candidate|SetInteractionCandidate (LocalVariables|GetNewInteractionCandidate)))
        (Default|CallOnInteractionCandidateChanged _output_get_2)))))

(fn Interact
  (if (!= (Variables|Candidate|GetInteractionCandidate) (Variables|Candidate|GetActiveInteraction))
    (Utilities|FlowControl|Sequence
      (:then_0
        (Interact|FinishInteraction))
      (:then_1
        (bind _interactioncandidate (Variables|Candidate|GetInteractionCandidate)
          (:then
            (bind _output_get (Variables|Candidate|SetActiveInteraction _interactioncandidate))
            (EventDispatchers|BindEventtoOnFinished _output_get (EventDispatchers|CreateEvent :!event ActiveInteractiononFinished))
            (Default|Interact (Variables|Candidate|GetActiveInteraction) self))
          (:else)))
      (:then_2
        (Candidate|DetermineInteractionCandidate))
      (:then_3
        (Default|CallOnActiveInteractionChanged (Variables|Candidate|GetActiveInteraction))))))

(fn FinishInteraction
  (bind _activeinteraction (Variables|Candidate|GetActiveInteraction)
    (:then
      (Default|FinishInteract _activeinteraction)
      (Variables|Candidate|SetActiveInteraction 0))
    (:else)))

(fn CollisiononComponentBeginOverlap
  (params (OverlappedComponent :type Primitive%20Component%20Object%20Reference) (OtherActor :type Actor%20Object%20Reference) (OtherComp :type Primitive%20Component%20Object%20Reference) (OtherBodyIndex :type Integer) (bFromSweep :type Boolean) (SweepResult :type Hit%20Result%20Structure%20%28by%20ref%29))
  (Utilities|Array|Add (Variables|Collision|GetInRangeInteractionActors) OtherActor)
  (Candidate|DetermineInteractionCandidate))

(fn CollisiononComponentEndOverlap
  (params (OverlappedComponent :type Primitive%20Component%20Object%20Reference) (OtherActor :type Actor%20Object%20Reference) (OtherComp :type Primitive%20Component%20Object%20Reference) (OtherBodyIndex :type Integer))
  (Utilities|Array|RemoveItem (Variables|Collision|GetInRangeInteractionActors) OtherActor)
  (Candidate|DetermineInteractionCandidate))

(fn ActiveInteractiononFinished
  (Variables|Candidate|SetActiveInteraction 0)
  (Candidate|DetermineInteractionCandidate))

(fn DetermineCollision
  (bind _array_element (Utilities|Array|ForEachLoopwithBreak (Components|GetChildrenComponents false))
    (:LoopBody
      (bind _asprimitive_component (Utilities|Casting|CastToPrimitiveComponent _array_element))
      (Variables|Collision|SetCollision _asprimitive_component))
    (:Completed
      (Variables|Collision|GetCollision
        (:then)
        (:else
          (Development|PrintString "ERROR: Interactor Component requires a child collision component to work." true true "(R=1.000000,G=0.000000,B=0.000000,A=1.000000)"))))))

(fn SetUpCollisionBindings
  (Utilities|FlowControl|Sequence
    (:then_0
      (Collision|BindEventtoOnComponentBeginOverlap (Variables|Collision|GetCollision) (EventDispatchers|CreateEvent :!event CollisiononComponentBeginOverlap)))
    (:then_1
      (Collision|BindEventtoOnComponentEndOverlap (Variables|Collision|GetCollision) (EventDispatchers|CreateEvent :!event CollisiononComponentEndOverlap)))))