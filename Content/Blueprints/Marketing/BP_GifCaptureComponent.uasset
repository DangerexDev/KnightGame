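; Actor component for marketing captures that records a render target to GIF files via a GifRecorder component it adds to its owner.
; ToggleRecording starts or stops recording from RT_GifCapture, naming each file by timestamp and saving into a gif folder under the project directory.
; Keyed on-screen messages report recording, saving and the final saved path, while red errors flag setup problems like a missing folder or wrong render target format.
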(fn ReceiveBeginPlay
  (|CallParentFunction)
  (bind _returnvalue (Game|AddComponentbyClass (Components|GetOwner) "/Script/GifRecorder.GifRecorderComponent"))
  (bind _output_get (Variables|Components|SetGifRecorderComponent _returnvalue))
  (Variables|/Script/GifRecorder.GifRecorderComponent|SetSaveDirectory _output_get (File|GetSaveDirectory))
  (EventDispatchers|BindEventtoOnSaved (Variables|Components|GetGifRecorderComponent) (EventDispatchers|CreateEvent :!event GifRecorderComponentonSaved)))

(fn GetFullFilePath
  (return (Utilities|String|Append (File|GetSaveDirectory) "\\" (File|GetFileName))))

(fn GetSaveDirectory
  (return (Utilities|String|Append (Utilities|String|Replace (Class|KismetSystemLibrary|GetProjectDirectory) "/" "\\") "gif")))

(fn GetFileName
  (return (Utilities|String|Append (File|GetDateTimeString) ".gif")))

(fn GetDateTimeString
  (bind _returnvalue (Math|DateTime|Now))
  (bind (_year _month _day _hour _minute _second _millisecond) (Math|DateTime|BreakDateTime _returnvalue))
  (return (Utilities|String|Append (Utilities|String|ToString(Integer) _year) "_" (Utilities|String|ToString(Integer) _month) "_" (Utilities|String|ToString(Integer) _day) "_" (Utilities|String|ToString(Integer) _hour) "_" (Utilities|String|ToString(Integer) _minute) "_" (Utilities|String|ToString(Integer) _second) "_" (Utilities|String|ToString(Integer) _millisecond))))

(fn DisplayErrorMessage
  (params (A :type String))
  (Development|PrintString (Utilities|String|Append A " File location was: " (File|GetFullFilePath)) true true "(R=1.000000,G=0.000000,B=0.000000,A=1.000000)" 5.0 "Error"))

(fn GifRecorderComponentonSaved
  (params (Path :type String))
  (Logging|DisplayRecordingStatusMessage (Utilities|String|Append "Saved recording to " Path) true))

(fn ToggleRecording
  (if (Variables|Recording|GetbRecording)
    (Recording|StopRecording)
    (else
      (Recording|StartRecording))))

(fn StartRecording
  (bind _returnvalue (Class|GifRecorderComponent|MakeGIF (Variables|Components|GetGifRecorderComponent) (File|GetFileName) "F25" 0 "/Game/Blueprints/Marketing/RT_GifCapture.RT_GifCapture"))
  (if _returnvalue
    (bind _returnvalue_2 (Class|GifRecorderComponent|RecordGIF (Variables|Components|GetGifRecorderComponent)))
    (bind _output_get (Variables|Recording|SetbRecording _returnvalue_2))
    (if _output_get
      (Logging|DisplayRecordingStatusMessage "Currently recording GIF..." false)
      (else
        (Logging|DisplayErrorMessage "Error starting GIF recording.")))
    (else
      (Logging|DisplayErrorMessage "Error creating GIF file. 
Possible issues: 
- You may need to add a folder named gif in the root of your project directory. 
- You may need to set the Render Target Format to RTF RGBA8."))))

(fn StopRecording
  (Class|GifRecorderComponent|StopRecordingGIF (Variables|Components|GetGifRecorderComponent))
  (Variables|Recording|SetbRecording false)
  (Logging|DisplayRecordingStatusMessage "Finished recording. Please wait for the GIF to save..." false))

(fn DisplayRecordingStatusMessage
  (params (InString :type String) (bIsFinal :type Boolean))
  (Development|PrintString InString true true "(R=0.000000,G=0.660000,B=1.000000,A=1.000000)" (select bIsFinal 2.0 3.6e+03) "RecordingStatus"))